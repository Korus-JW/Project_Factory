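; Base actor for factory buildings, handling placement preview and demolition highlight visuals, build cost setup and rotation requests.
; On BeginPlay it creates a dynamic preview material, tinted green or red by buildability and red for demolition.
; Highlighting disallows Nanite on static meshes, caches each mesh's materials and overrides slot 0.
; Releasing the highlight re-allows Nanite and restores the cached materials.
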(event Custom|Rotate
  (Class|FactoryBuildingBase|RotateBuilding))

(event Custom|Destruction%20Hightlight
  (Rendering|Material|SetVectorParameterValue (Variables|Default|GetPreview%20Material) "Preview Color" "(R=1.000000,G=0.000000,B=0.000000,A=1.000000)" :!class /Script/Engine.MaterialInstanceDynamic)
  (CallFunction|OnOffNanite (Variables|Mesh|GetBuilding%20Meshes) true)
  (CallFunction|PreviewHighlight (Variables|Mesh|GetBuilding%20Meshes) (Variables|Default|GetPreview%20Material)))

(event Custom|Release%20Destruction%20Highlight
  (CallFunction|OnOffNanite (Variables|Mesh|GetBuilding%20Meshes) false)
  (CallFunction|ReleasePreviewHighlight))

(event EventBeginPlay
  (bind _returnvalue (Rendering|Material|CreateDynamicMaterialInstance "/Game/Resource/Preview/MI_Preview.MI_Preview" "None" "None" :!class /Script/Engine.KismetMaterialLibrary))
  (Variables|Default|SetPreview%20Material _returnvalue)
  (Variables|Default|SetBuildCost (.cost (Variables|Default|GetInfo))))

(event Collision|EventActorBeginOverlap
  (params (OtherActor :type Actor%20Object%20Reference)))

(event EventTick
  (params (DeltaSeconds :type Float%20%28single-precision%29)))

(event EventOnCanBuildChanged
  (params (bChangedCanBuild :type Boolean))
  (bind _preview_material (Variables|Default|GetPreview%20Material))
  (if bChangedCanBuild
    (Rendering|Material|SetVectorParameterValue _preview_material "Preview Color" "(R=0.000000,G=1.000000,B=0.000000,A=1.000000)" :!class /Script/Engine.MaterialInstanceDynamic)
    (else
      (Rendering|Material|SetVectorParameterValue _preview_material "Preview Color" "(R=1.000000,G=0.000000,B=0.000000,A=1.000000)" :!class /Script/Engine.MaterialInstanceDynamic))))

(event EventOnPlacementPreviewChanged
  (params (bPreview :type Boolean))
  (bind _building_meshes (Variables|Mesh|GetBuilding%20Meshes))
  (if bPreview
    ;[0.0185 0.15 0.02381 0.5] 프리뷰 머터리얼로 변경
    (CallFunction|OnOffNanite _building_meshes true)
    (CallFunction|PreviewHighlight _building_meshes (Variables|Default|GetPreview%20Material))
    (else
      ;[0.15 0.01798 0.01992 0.5] 원래 머터리얼로 복원
      (CallFunction|OnOffNanite (Variables|Mesh|GetBuilding%20Meshes) false)
      (CallFunction|ReleasePreviewHighlight))))

(fn ConstructionScript)

(fn PreviewHighlight
  (params (Meshes :type Array%20of%20Static%20Mesh%20Component%20Object%20References) (Material :type Material%20Interface%20Object%20Reference))
  (Utilities|Array|Clear (Variables|Default|GetOriginalMaterial))
  (for _array_element Meshes
    (Utilities|Array|Add (Variables|Default|GetOriginalMaterial) (Utilities|Struct|MakeST_BackupMaterial _array_element (Rendering|Material|GetMaterials _array_element)))
    (Rendering|Material|SetMaterial _array_element 0 Material)))

(fn OnOffNanite
  (params (Meshes :type Array%20of%20Primitive%20Component%20Object%20References) (나나이트%20불허 :type Boolean))
  (for _array_element Meshes
    (bind _as스태틱_메시_컴포넌트 (Utilities|Casting|CastToStaticMeshComponent _array_element))
    (Variables|/Script/Engine.StaticMeshComponent|SetbDisallowNanite _as스태틱_메시_컴포넌트 나나이트%20불허)))

(fn ReleasePreviewHighlight
  (for _array_element (Variables|Default|GetOriginalMaterial)
    (for (_array_element_2 _array_index) (.material _array_element)
      (Rendering|Material|SetMaterial (.mesh _array_element) _array_index _array_element_2))))