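; BP_Processing is a processing building Blueprint, with factory, storage room and road meshes, that builds on the logic of its parent class.
; On BeginPlay it runs the parent logic, then appends its building, factory, two storage room, and enter and exit road meshes to the BuildingMeshes array.
; The construction script only calls the parent, and the overlap and tick events are disabled.
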(event EventBeginPlay
  (|CallParentFunction)
  (Utilities|Array|AppendArray (Variables|Default|GetBuilding%20Meshes) (Utilities|Array|MakeArray (Variables|Default|GetBuildingMesh) (Variables|Default|GetSM_Factory_Storage_room) (Variables|Default|GetFactory) (Variables|Default|GetSM_Factory_Storage_room1) (Variables|Default|GetEnterRoad) (Variables|Default|GetExit%20Road))))

(event Collision|EventActorBeginOverlap
  (params (OtherActor :type Actor%20Object%20Reference))
  (|CallParentFunction OtherActor) ; 지금 이 노드는 비활성 상태입니다. \n핀을 끌어서 다른 노드를 연결하면 활성화됩니다.
)

(event EventTick
  (params (DeltaSeconds :type Float%20%28single-precision%29))
  (|CallParentFunction DeltaSeconds) ; 지금 이 노드는 비활성 상태입니다. \n핀을 끌어서 다른 노드를 연결하면 활성화됩니다.
)

(fn ConstructionScript
  (|CallParentFunction))