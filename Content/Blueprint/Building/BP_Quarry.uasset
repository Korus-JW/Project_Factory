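; BP_Quarry is a quarry building Blueprint that registers its factory mesh parts with logic inherited from a parent class.
; On BeginPlay it runs the parent logic, then appends the main building, refinery, warehouse and administration meshes to BuildingMeshes.
; It also appends the enter and exit road meshes to RoadMeshes.
; The overlap and Tick events and the construction script are empty.
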(event EventBeginPlay
  (|CallParentFunction)
  (Utilities|Array|AppendArray (Variables|Default|GetBuilding%20Meshes) (Utilities|Array|MakeArray (Variables|Default|GetBuildingMesh) (Variables|Default|GetSM_Factory_Refinery_01) (Variables|Default|GetSM_Factory_Warehouse_01) (Variables|Default|GetSM_Factory_Warehouse_02) (Variables|Default|GetSM_Factory_Administration_03)))
  (Utilities|Array|AppendArray (Variables|Default|GetRoad%20Meshes) (Utilities|Array|MakeArray (Variables|Default|GetSM_Factory_Enter_Road) (Variables|Default|GetSM_Factory_Exit_Road))))

(event Collision|EventActorBeginOverlap
  (params (OtherActor :type Actor%20Object%20Reference)))

(event EventTick
  (params (DeltaSeconds :type Float%20%28single-precision%29)))

(fn ConstructionScript)