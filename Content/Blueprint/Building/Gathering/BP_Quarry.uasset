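; BP_Quarry is a gathering building Blueprint for a quarry, with animated drills.
; On BeginPlay it runs the parent logic, then appends its administration, drill, tank and road meshes plus the main mesh to the inherited BuildingMeshes array.
; Tick spins both drill rotors by a fixed relative rotation each frame, not scaled by delta time.
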(event EventBeginPlay
  (|CallParentFunction)
  (Utilities|Array|AppendArray (Variables|Default|GetBuilding%20Meshes) (Utilities|Array|MakeArray (Variables|Default|GetBuildingMesh) (Variables|Default|GetSM_Factory_Administration_01) (Variables|Default|GetSM_QuarryDrill_Base_300) (Variables|Default|GetSM_QuarryDrill_Rotor_300) (Variables|Default|GetSM_Factory_Tank_01) (Variables|Default|GetSM_QuarryDrill_Base_301) (Variables|Default|GetSM_QuarryDrill_Rotor_301) (Variables|Default|GetSM_Factory_Enter_Road) (Variables|Default|GetSM_Factory_Exit_Road))))

(event Collision|EventActorBeginOverlap
  (params (OtherActor :type Actor%20Object%20Reference)))

(event EventTick
  (params (DeltaSeconds :type Float%20%28single-precision%29))
  (Transformation|AddRelativeRotation (Variables|Default|GetSM_QuarryDrill_Rotor_300) "0.000000,15.000000,0.000000" false false))

(fn ConstructionScript)