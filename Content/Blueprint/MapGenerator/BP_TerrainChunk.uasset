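; Terrain chunk actor that renders a grid of land, water, wood and stone as instanced static meshes.
; On BeginPlay it has TerrainWorldSubsystem generate a test chunk, then adds instances per cell, mapping resource cells to instance indices.
; It also binds to the subsystem's cell occupancy event.
; OnCellChanged hides resources under buildings by scaling instances to zero and restores them when clear, keeping stored indices stable.
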(event EventBeginPlay
  (bind _returnvalue (Subsystems|GetTerrainWorldSubsystem))
  (bind _chunk_coordinate (Variables|Default|GetChunk%20Coordinate))
  (bind _outdata (Class|TerrainWorldSubsystem|GetChunk _returnvalue _chunk_coordinate))
  (EventDispatchers|BindEventtoOnCellOccupancyChanged _returnvalue (EventDispatchers|CreateEvent :!event OnCellChanged))
  (Class|TerrainWorldSubsystem|GenerateTestChunk _returnvalue (Variables|Default|GetChunk%20Coordinate) 100 100 4 true)
  (if true
    (Components|InstancedStaticMesh|ClearInstances (Variables|Default|GetISM_Land))
    (Variables|Default|SetWidth (.width _outdata))
    (for (_array_element _array_index) (.cells _outdata)
      (switch Utilities|FlowControl|Switch|SwitchonETerrainType (.terraintype _array_element)
        (:Land
          (Components|InstancedStaticMesh|AddInstance (Variables|Default|GetISM_Land) (Math|Transform|MakeTransform (Class|TerrainDataLibrary|GetCellLocalOrigin (Math|Integer|%(Integer) _array_index (Variables|Default|GetWidth)) (/ _array_index (Variables|Default|GetWidth))) "0, 0, 0" "1.000000,1.000000,1.000000") true)
          (switch Utilities|FlowControl|Switch|SwitchonECellResourceType (.resourcetype _array_element)
            (:Wood
              (bind _returnvalue_2 (Components|InstancedStaticMesh|AddInstance (Variables|Default|GetISM_Wood) (Math|Transform|MakeTransform (+ (Class|TerrainDataLibrary|GetCellLocalOrigin (Math|Integer|%(Integer) _array_index (Variables|Default|GetWidth)) (/ _array_index (Variables|Default|GetWidth))) "250.000000,250.000000,0.000000") "0, 0, 0" "1.000000,1.000000,1.000000") true))
              (Utilities|Map|Add (Variables|Default|GetResource%20Instance) (Utilities|Struct|MakeIntPoint (Math|Integer|%(Integer) _array_index (Variables|Default|GetWidth)) (/ _array_index (Variables|Default|GetWidth))) _returnvalue_2))
            (:Stone
              (bind _returnvalue_3 (Components|InstancedStaticMesh|AddInstance (Variables|Default|GetISM_Stone) (Math|Transform|MakeTransform (+ (Class|TerrainDataLibrary|GetCellLocalOrigin (Math|Integer|%(Integer) _array_index (Variables|Default|GetWidth)) (/ _array_index (Variables|Default|GetWidth))) "250.000000,250.000000,0.000000") "0, 0, 0" "1.000000,1.000000,1.000000") true))
              (Utilities|Map|Add (Variables|Default|GetResource%20Instance) (Utilities|Struct|MakeIntPoint (Math|Integer|%(Integer) _array_index (Variables|Default|GetWidth)) (/ _array_index (Variables|Default|GetWidth))) _returnvalue_3))))
        (:Water
          (Components|InstancedStaticMesh|AddInstance (Variables|Default|GetISM_Water) (Math|Transform|MakeTransform (Class|TerrainDataLibrary|GetCellLocalOrigin (Math|Integer|%(Integer) _array_index (Variables|Default|GetWidth)) (/ _array_index (Variables|Default|GetWidth))) "0, 0, 0" "1.000000,1.000000,1.000000") true))))
    (else
      (Development|PrintString "Fail"))))

(event Collision|EventActorBeginOverlap
  (params (OtherActor :type Actor%20Object%20Reference)))

(event EventTick
  (params (DeltaSeconds :type Float%20%28single-precision%29)))

(fn ConstructionScript)

(fn OnCellChanged
  (params (ChangedCells :type Array%20of%20Int%20Point%20Structures))
  (bind _ism_stone (Variables|Default|GetISM_Stone))
  (bind _ism_wood (Variables|Default|GetISM_Wood))
  (for _array_element ChangedCells
    (LocalVariables|SetCurrent%20Cell _array_element)
    (if (.ReturnValue (Class|TerrainWorldSubsystem|GetCell (Subsystems|GetTerrainWorldSubsystem) (Variables|Default|GetChunk%20Coordinate) (.x (LocalVariables|GetCurrent%20Cell)) (.y (LocalVariables|GetCurrent%20Cell))))
      (if (.ReturnValue (Utilities|Map|Find (Variables|Default|GetResource%20Instance) (LocalVariables|GetCurrent%20Cell)))
        (Utilities|IsValid (Class|TerrainWorldSubsystem|GetBuildingatCell (Subsystems|GetTerrainWorldSubsystem) (LocalVariables|GetCurrent%20Cell))
          (:Is%20Valid
            (switch Utilities|FlowControl|Switch|SwitchonECellResourceType (.resourcetype (.OutCell (Class|TerrainWorldSubsystem|GetCell (Subsystems|GetTerrainWorldSubsystem) (Variables|Default|GetChunk%20Coordinate) (.x (LocalVariables|GetCurrent%20Cell)) (.y (LocalVariables|GetCurrent%20Cell)))))
              (:Wood
                (Components|InstancedStaticMesh|UpdateInstanceTransform _ism_wood (.Value (Utilities|Map|Find (Variables|Default|GetResource%20Instance) (LocalVariables|GetCurrent%20Cell))) (Math|Transform|MakeTransform (.Location (Math|Transform|BreakTransform (.OutInstanceTransform (Components|InstancedStaticMesh|GetInstanceTransform _ism_wood (.Value (Utilities|Map|Find (Variables|Default|GetResource%20Instance) (LocalVariables|GetCurrent%20Cell))) false)))) (.Rotation (Math|Transform|BreakTransform (.OutInstanceTransform (Components|InstancedStaticMesh|GetInstanceTransform _ism_wood (.Value (Utilities|Map|Find (Variables|Default|GetResource%20Instance) (LocalVariables|GetCurrent%20Cell))) false)))) "0,0,0") false true true))
              (:Stone
                (Components|InstancedStaticMesh|UpdateInstanceTransform _ism_stone (.Value (Utilities|Map|Find (Variables|Default|GetResource%20Instance) (LocalVariables|GetCurrent%20Cell))) (Math|Transform|MakeTransform (.Location (Math|Transform|BreakTransform (.OutInstanceTransform (Components|InstancedStaticMesh|GetInstanceTransform _ism_stone (.Value (Utilities|Map|Find (Variables|Default|GetResource%20Instance) (LocalVariables|GetCurrent%20Cell))) false)))) (.Rotation (Math|Transform|BreakTransform (.OutInstanceTransform (Components|InstancedStaticMesh|GetInstanceTransform _ism_stone (.Value (Utilities|Map|Find (Variables|Default|GetResource%20Instance) (LocalVariables|GetCurrent%20Cell))) false)))) "0,0,0") false true true))))
          (:Is%20Not%20Valid
            (switch Utilities|FlowControl|Switch|SwitchonECellResourceType (.resourcetype (.OutCell (Class|TerrainWorldSubsystem|GetCell (Subsystems|GetTerrainWorldSubsystem) (Variables|Default|GetChunk%20Coordinate) (.x (LocalVariables|GetCurrent%20Cell)) (.y (LocalVariables|GetCurrent%20Cell)))))
              (:Wood
                (Components|InstancedStaticMesh|UpdateInstanceTransform _ism_wood (.Value (Utilities|Map|Find (Variables|Default|GetResource%20Instance) (LocalVariables|GetCurrent%20Cell))) (Math|Transform|MakeTransform (.Location (Math|Transform|BreakTransform (.OutInstanceTransform (Components|InstancedStaticMesh|GetInstanceTransform _ism_wood (.Value (Utilities|Map|Find (Variables|Default|GetResource%20Instance) (LocalVariables|GetCurrent%20Cell))) false)))) (.Rotation (Math|Transform|BreakTransform (.OutInstanceTransform (Components|InstancedStaticMesh|GetInstanceTransform _ism_wood (.Value (Utilities|Map|Find (Variables|Default|GetResource%20Instance) (LocalVariables|GetCurrent%20Cell))) false)))) "1,1,1") false true true))
              (:Stone
                (Components|InstancedStaticMesh|UpdateInstanceTransform _ism_stone (.Value (Utilities|Map|Find (Variables|Default|GetResource%20Instance) (LocalVariables|GetCurrent%20Cell))) (Math|Transform|MakeTransform (.Location (Math|Transform|BreakTransform (.OutInstanceTransform (Components|InstancedStaticMesh|GetInstanceTransform _ism_stone (.Value (Utilities|Map|Find (Variables|Default|GetResource%20Instance) (LocalVariables|GetCurrent%20Cell))) false)))) (.Rotation (Math|Transform|BreakTransform (.OutInstanceTransform (Components|InstancedStaticMesh|GetInstanceTransform _ism_stone (.Value (Utilities|Map|Find (Variables|Default|GetResource%20Instance) (LocalVariables|GetCurrent%20Cell))) false)))) "1,1,1") false true true)))))))))