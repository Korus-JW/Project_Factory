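; BP_FactoryCharacter is a player-controlled camera character that moves freely and zooms its spring arm.
; Move input offsets the actor along its forward and right vectors without sweep or delta-time scaling, using a step size that MoveScale input adjusts within a clamped range.
; Zoom input sets a clamped target arm length, which Tick smoothly interpolates the SpringArm toward.
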(event EventBeginPlay)

(event Collision|EventActorBeginOverlap
  (params (OtherActor :type Actor%20Object%20Reference)))

(event EventTick
  (params (DeltaSeconds :type Float%20%28single-precision%29))
  (bind _springarm (Variables|Default|GetSpringArm))
  (Variables|/Script/Engine.SpringArmComponent|SetTargetArmLength _springarm (Math|Interpolation|FInterpTo (Variables|/Script/Engine.SpringArmComponent|GetTargetArmLength _springarm) (Variables|이동|GetTarget%20Zoom%20Scale) DeltaSeconds 3.0)))

(event Custom|Move
  (params (Input :type Vector%202D%20Structure))
  (bind _movement_scale (Variables|Movement|GetMovement%20Scale))
  (Transformation|AddActorWorldOffset (+ (* (* (Transformation|GetActorForwardVector) (.x Input)) _movement_scale) (* (* (Transformation|GetActorRightVector) (.y Input)) _movement_scale))))

(event Custom|Move%20Scale
  (params (Input :type Float%20%28double-precision%29))
  (Variables|Movement|SetMovement%20Scale (Math|Float|Clamp(Float) (+ (* Input 5e+01) (Variables|Movement|GetMovement%20Scale)) 5e+01 1.5e+02)))

(event Custom|Zoom
  (params (Input :type Float%20%28double-precision%29))
  (Variables|이동|SetTarget%20Zoom%20Scale (Math|Float|Clamp(Float) (+ (Variables|이동|GetTarget%20Zoom%20Scale) (* Input 1e+03)) 0.0 4e+03)))

(fn ConstructionScript)